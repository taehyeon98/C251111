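; BP_GameMode is a game mode Blueprint that advances the game to the next level once the stage's targets are gone.
; Its NextStage event checks for remaining actors tagged "Target"; when none exist, it prints a next-map message and waits briefly.
; It then reads the next level name from the first BP_Stage actor and opens that level.
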(event Custom|NextStage
  (bind _outactors (Actor|GetAllActorswithTag "Target"))
  (if (== (Utilities|Array|Length _outactors) 0)
    (Development|PrintString "다음맵으로")
    (Utilities|FlowControl|Delay 3.0)
    (bind _outactors_2 (Actor|GetAllActorsOfClass "/Game/Blueprint/BP_Stage.BP_Stage_C"))
    (Game|OpenLevel(byName) (Utilities|String|StringToName (Variables|/Game/Blueprint/BP_Stage.BP_Stage_C|GetNextStage (Utilities|Array|Get(acopy) _outactors_2))))))

(fn ConstructionScript)