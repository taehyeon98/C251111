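; BP_Rocket is a short-lived projectile actor that expires a few seconds after spawning.
; On overlapping an actor tagged Target, it applies damage credited to the first player controller, plays explosion sound and particles, and destroys itself.
; It then casts the game mode to BP_GameMode and calls NextStage, so each target hit triggers a stage advance.
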(event EventBeginPlay
  (Actor|SetLifeSpan 3.0))

(event Collision|EventActorBeginOverlap
  (params (OtherActor :type Actor%20Object%20Reference))
  (if (Actor|ActorHasTag OtherActor "Target")
    (Game|Damage|ApplyDamage OtherActor 1e+01 (Game|GetPlayerController 0) self)
    (Audio|SpawnSoundatLocation "/Game/StarterContent/Audio/Explosion_Cue.Explosion_Cue" (Transformation|GetActorLocation) "0, 0, 0" 1.0 1.0 0.0 0 0)
    (Effects|SpawnEmitteratLocation "/Game/StarterContent/Particles/P_Explosion.P_Explosion" (Transformation|GetActorLocation))
    (Actor|DestroyActor)
    (bind _asbp_game_mode (Utilities|Casting|CastToBP_GameMode (Game|GetGameMode)))
    (Default|NextStage _asbp_game_mode)))

(fn ConstructionScript)